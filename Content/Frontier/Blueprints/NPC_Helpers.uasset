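; NPC_Helpers is a set of helper functions for NPC faction combat and target resolution.
; Factions count as fighting whenever they differ.
; The fighting-actor query gathers every BP_NPC of an opposing faction, adding the player character only when one specific faction is passed in.
; A cast helper resolves a blackboard target into either BP_FPSCharacter or BP_NPC, with flags for which it is.
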(fn `BB Target Reference to Player or NPC`
  (params (Target :type "Object Object Reference"))
  (returns (Player :type "/Game/Frontier/Blueprints/BP_FPSCharacter Object Reference") (NPC :type "/Game/Frontier/Blueprints/BP_NPC Object Reference") (`Is Player` :type Boolean) (`Is NPC` :type Boolean))
  (bind _asbp_fpscharacter (cast `/Game/Frontier/Blueprints/BP_FPSCharacter` Target)
    (:`then`
      (return _asbp_fpscharacter null true false))
    (:`CastFailed`
      (bind _asbp_npc (cast `/Game/Frontier/Blueprints/BP_NPC` Target)
        (:`then`
          (return null _asbp_npc false true))
        (:`CastFailed`
          (if false
            (`KismetSystemLibrary.PrintString` null "Faild to get player or NPC from cast!")))))))

(fn `DoseFactionFight`
  (params (faction1 :type "/Game/Frontier/Art/Faction Enum" :default "NewEnumerator0") (faction2 :type "/Game/Frontier/Art/Faction Enum" :default "NewEnumerator0"))
  (returns (doseFactionFight :type Boolean))
  (return (`|EnumInequality` faction1 faction2)))

(fn `Get Fighting Actors Of Faction`
  (params (faction :type "/Game/Frontier/Art/Faction Enum" :default "NewEnumerator0"))
  (returns (`Fighting Actors` :type "Array of Actor Object Reference"))
  (locals (fightingActors :type "Array of Actor Object Reference"))
  (bind _returnvalue (`GameplayStatics.GetPlayerCharacter` null))
  ;[1 1 1] Add Player to fighting Actors
  (if (`|EnumEquality` "NewEnumerator1" faction)
    (`/Engine/EditorBlueprintResources/StandardMacros.IsValid` _returnvalue
      (:`Is Valid`
        (`KismetArrayLibrary.Array_Add` (`local.fightingActors`) _returnvalue))
      (:`Is Not Valid`
        _)))
  (bind _outactors (`GameplayStatics.GetAllActorsOfClass` null "/Game/Frontier/Blueprints/BP_NPC.BP_NPC_C"))
  (for _array_element _outactors
    (bind _dosefactionfight (`self.DoseFactionFight` (`/Game/Frontier/Blueprints/BP_NPC.faction` _array_element) faction))
    (if _dosefactionfight
      (`KismetArrayLibrary.Array_Add` (`local.fightingActors`) _array_element)))
  (return (`local.fightingActors`)))