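; NPC character that takes point damage and dies with a montage-to-ragdoll transition.
; Each hit launches it along the shot direction, then, if it is still alive, subtracts health and plays a pistol hit montage or triggers Death.
; Death stops movement and plays a death montage whose notify enables physics on all mesh bodies.
; The run-to-player AI move loop is disconnected, so no chasing happens here.
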(event `self.ReceiveBeginPlay`
  (`self.RunToPlayer_Event`))

(event `RunToPlayer_Event`
  ;[1 1 1] Run to player
)

(event `self.ReceivePointDamage`
  (params (Damage :type "Float (single-precision)") (DamageType :type "DamageType Object Reference") (HitLocation :type "Vector Structure") (HitNormal :type "Vector Structure") (HitComponent :type "PrimitiveComponent Object Reference") (BoneName :type Name) (ShotFromDirection :type "Vector Structure") (InstigatedBy :type "Controller Object Reference") (DamageCauser :type "Actor Object Reference") (HitInfo :type "HitResult Structure (by ref)"))
  ;[1 1 1] Get Shot
  (`self.LaunchCharacter` (* (`KismetMathLibrary.GetDirectionUnitVector` HitInfo_TraceStart HitInfo_TraceEnd) (2000.0 2000.0 2000.0)))
  (bind _isdead (`self.IsDead`))
  (if (not _isdead)
    ;;[1 1 1] For some reason this was reqired at one point. It stays here just in case it returns.
    (bind _output_get (set `self.health` (- (`self.health`) Damage)))
    (set `self.beenShot` true)
    (`KismetSystemLibrary.PrintString` (`KismetStringLibrary.Concat_StrStr` "NPC health is:" (`KismetStringLibrary.Conv_DoubleToString` (`self.health`)) "And dammage is" (`KismetStringLibrary.Conv_DoubleToString` Damage)) true true (struct :`G` 0.66 :`B` 1.0 :`A` 1.0) 10.0)
    (if (<= _output_get 0.0)
      (`self.Death`)
      (else
        (`|PlayMontage` (`self.Mesh`) "/Game/NPC/Animations/AM_Pistol_Hit.AM_Pistol_Hit")))))

(event `Death`
  ;[1 1 1] Death
  (`MovementComponent.StopMovementImmediately` (`self.CharacterMovement`))
  (`|PlayMontage` (`self.Mesh`) "/Game/NPC/Animations/AM_Generic_Death.AM_Generic_Death"
    (:`then`
      (`KismetSystemLibrary.PrintString` "Final Dead"))
    (:`OnNotifyBegin`
      (`SkeletalMeshComponent.SetAllBodiesSimulatePhysics` (`self.Mesh`) true))))

(fn `IsDead`
  (returns (isDead :type Boolean))
  (return (<= (`self.health`) 0.0)))

(fn `UserConstructionScript`)